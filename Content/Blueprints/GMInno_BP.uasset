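; Game mode for an online Innovation ("Inno") card game client that talks to a web server over HTTP.
; On BeginPlay it logs in, scrapes the session token from the play page's inline script, then long-polls, feeding responses to InnoTick.
; Lobby reset and hide events swap lobby and game widgets through paired DoOnce gates.
; Library events send chat, game proposals and replies as JSON, fetch card data and sign out on EndPlay.
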(event `self.ReceiveBeginPlay`
  (add `Requester.OnLightRequestResponse` (`self.Requester`) (delegate `LightResponse`))
  (add `self.Inno_Cards` (`|CreateDelegate` :!event `InnoCards`))
  (`self.Begin`))

(event `LightResponse`
  (params (Code :type Integer) (Content :type String) (bWasSuccessful :type Boolean))
  (`self.InnoTick` Content))

(event `Begin`
  (`Requester.Request` (`self.Requester`) (delegate `OnLogin`) "notloggedin" "POST" ""))

(event `OnLogin`
  (params (Code :type Integer) (Content :type String) (bWasSuccessful :type Boolean))
  (if bWasSuccessful
    (`Requester.Request` (`self.Requester`) (delegate `OnLobby`) "notloggedin" "POST" (`self.BuildLoginData`))
    (`KismetSystemLibrary.Delay` 2.0)
    (`Requester.Request` (`self.Requester`) (delegate `OnPlay`) "play" "GET" "")
    (else
      (`KismetSystemLibrary.PrintString` "Fail"))))

(event `OnLobby`
  (params (Code :type Integer) (Content :type String) (bWasSuccessful :type Boolean))
  (`KismetSystemLibrary.PrintString` "Unable to login. Username is taken?" :!label _label))

(event `OnPlay`
  (params (Code :type Integer) (Content :type String) (bWasSuccessful :type Boolean))
  (bind _returnvalue (`GameplayStatics.GetPlayerController` 0))
  (`KismetSystemLibrary.PrintString` (`KismetStringLibrary.Conv_BoolToString` bWasSuccessful))
  (bind _output_get (set `self.BrowserToken` (`InnoFunctionLibrary.GetInlineScriptVar` Content "BROWSER_TOKEN")))
  (bind _output_get_2 (set `self.StaticDir` (`InnoFunctionLibrary.GetInlineScriptVar` Content "STATIC_DIR")))
  (if (and (`KismetStringLibrary.NotEqual_StrStr` _output_get) (`KismetStringLibrary.NotEqual_StrStr` _output_get_2))
    (`KismetSystemLibrary.PrintText` (`|FormatText` "Token: {Token}, Dir: {Dir}" (`KismetTextLibrary.Conv_StringToText` _output_get) (`KismetTextLibrary.Conv_StringToText` _output_get_2)))
    (`self.BeginLobbyLoop`)
    (bind _returnvalue_2 (`|CreateWidget` "/Game/Widgets/Lobby/W_Lobby.W_Lobby_C" _returnvalue))
    (bind _output_get_3 (set `self.WidgetLobby` _returnvalue_2))
    (bind _returnvalue_3 (`|CreateWidget` "/Game/Widgets/Game/W_Game.W_Game_C" _returnvalue))
    (set `self.WidgetGame` _returnvalue_3)
    (`WidgetBlueprintLibrary.SetInputMode_UIOnlyEx` (`GameplayStatics.GetPlayerController` 0) _output_get_3)
    (add `self.Lobby_Reset` (delegate `OnShowLobby`))
    (add `self.HideLobby` (delegate `OnHideLobby`))
    (else
      (goto _label))))

(event `OnShowLobby`
  (`/Engine/EditorBlueprintResources/StandardMacros.DoOnce` false :!label _label_2
    (:`Completed`
      (`Widget.RemoveFromParent` (`self.WidgetGame`))
      (`UserWidget.AddToPlayerScreen` (`self.WidgetLobby`) 0)
      (goto _label_3 :!via `Reset`))))

(event `OnHideLobby`
  (`/Engine/EditorBlueprintResources/StandardMacros.DoOnce` true :!label _label_3
    (:`Completed`
      (`Widget.RemoveFromParent` (`self.WidgetLobby`))
      (`UserWidget.AddToPlayerScreen` (`self.WidgetGame`) 0)
      (goto _label_2 :!via `Reset`))))

(event `self.ReceiveEndPlay`
  (params (EndPlayReason :type "EEndPlayReason Enum" :default "Destroyed"))
  (`self.Logout`))

(event `SendMessage`
  (params (Message :type String))
  ;[1 1 1] Chat
  (`Requester.LightRequest` (`self.Requester`) (`KismetStringLibrary.Concat_StrStr` "request/" (`self.BrowserToken`)) (`KismetStringLibrary.Concat_StrStr` "{\"type\":\"text\",\"entry\":\"" Message "\",\"shout\":false}")))

(event `ProposeGame`
  (params (OtherPlayers :type "Set of String") (Echoes :type Boolean) (Figures :type Boolean) (Cities :type Boolean) (ExtraAchievement :type Boolean))
  ;[1 1 1] Propose
  (bind _result (`BlueprintSetLibrary.Set_ToArray` OtherPlayers))
  (`Requester.LightRequest` (`self.Requester`) (`KismetStringLibrary.Concat_StrStr` "reply/" (`self.BrowserToken`)) (`self.BuildProposeJson` _result Echoes Figures Cities ExtraAchievement)))

(event `Logout`
  ;[1 1 1] Logout
  (`Requester.Request` (`self.Requester`) (delegate `Nop`) "signout" "GET" ""))

(event `Nop`
  (params (Code :type Integer) (Content :type String) (bWasSuccessful :type Boolean))
  ;[1 1 1] Logout
)

(event `BeginLobbyLoop`
  (`self.LobbyLoop` 0 "" true))

(event `Reply`
  (params (RequestId :type Integer) (Answer :type "Array of String"))
  ;[1 1 1] Reply
  (`Requester.LightRequest` (`self.Requester`) (`KismetStringLibrary.Concat_StrStr` "reply/" (`self.BrowserToken`)) (`self.BuildReplyJson` RequestId Answer)))

(event `LobbyLoop`
  (params (Code :type Integer) (Content :type String) (bWasSuccessful :type Boolean))
  (if bWasSuccessful
    (bind _returnvalue (`self.InnoTick` Content))
    (if _returnvalue
      (`Requester.Request` (`self.Requester`) (delegate `LobbyLoop`) (`KismetStringLibrary.Concat_StrStr` "wait/" (`self.BrowserToken`) "/" (`KismetStringLibrary.Conv_IntToString` (`self.LobbyLoopNextRequestId`))) "GET" "")
      (else
        (`KismetSystemLibrary.PrintString` Content)))
    (else
      (`KismetSystemLibrary.PrintString` "Lobby loop failed!"))))

(event `InnoCards`
  (params (CardsURL :type String))
  (`Requester.GetPage` (`self.Requester`) (delegate `UpdateCards`) CardsURL))

(event `UpdateCards`
  (params (Code :type Integer) (Content :type String) (bWasSuccessful :type Boolean))
  (if bWasSuccessful
    (`InnoCards.Update` (`self.Cards`) Content)))

(fn `GetChatWidget`
  (returns (`Chat Widget` :type "/Game/Widgets/W_Chat Object Reference"))
  (`/Engine/EditorBlueprintResources/StandardMacros.IsValid` (`self.WidgetChat`)
    (:`Is Valid`
      _)
    (:`Is Not Valid`
      (bind _returnvalue (`|CreateWidget` "/Game/Widgets/W_Chat.W_Chat_C"))
      (bind _output_get (set `self.WidgetChat` _returnvalue))))
  (return _output_get))

(fn `GetLogWidget`
  (returns (`Chat Widget` :type "/Game/Widgets/W_Log Object Reference"))
  (`/Engine/EditorBlueprintResources/StandardMacros.IsValid` (`self.WidgetLog`)
    (:`Is Valid`
      _)
    (:`Is Not Valid`
      (bind _returnvalue (`|CreateWidget` "/Game/Widgets/W_Log.W_Log_C"))
      (bind _output_get (set `self.WidgetLog` _returnvalue))))
  (return _output_get))

(fn `UserConstructionScript`)